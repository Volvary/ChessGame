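; BP_BoardTile is a chess board tile that shows its square color and a selection marker, and reports clicks.
; ChangeColor picks white or black from the parity of Position and maps SelectionState to a marker material for selection, move, capture, castling or failure feedback.
; The marker starts hidden and also hides for the None and Threaten states.
; ActorOnClicked passes the tile itself to CallOnTileClicked.
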(event EventBeginPlay
  (Development|SetHiddeninGame (Variables|Default|GetMarkerMesh) true false))

(event EventChangeColor
  (bind _position (Variables|Default|GetPosition))
  (bind _selectionstate (Variables|Default|GetSelectionState))
  (Rendering|Material|SetMaterial (Variables|Default|GetMesh) 0 (select (Class|KismetMathLibrary|XORBoolean (Math|Conversions|ToBoolean(Integer) (Math|Integer|%(Integer) (.x _position) 2)) (Math|Conversions|ToBoolean(Integer) (Math|Integer|%(Integer) (.y _position) 2))) "/Game/ChessGame/Materials/Tile_White.Tile_White" "/Game/ChessGame/Materials/Tile_Black.Tile_Black"))
  (Rendering|Material|SetMaterial (Variables|Default|GetMarkerMesh) 0 (Utilities|Select :Index (Variables|Default|GetSelectionState) :None "/Game/ChessGame/Materials/TileSelection.TileSelection" :Clicked "/Game/ChessGame/Materials/TileSelection_Selection.TileSelection_Selection" :ClickedWaiting "/Game/ChessGame/Materials/TileSelection_SelectionWaiting.TileSelection_SelectionWaiting" :ValidMove "/Game/ChessGame/Materials/TileSelection_ValidMove.TileSelection_ValidMove" :ValidMoveWaiting "/Game/ChessGame/Materials/TileSelection_ValidMoveWaiting.TileSelection_ValidMoveWaiting" :Capture "/Game/ChessGame/Materials/TileSelection_Capture.TileSelection_Capture" :CaptureWaiting "/Game/ChessGame/Materials/TileSelection_CaptureWaiting.TileSelection_CaptureWaiting" :NonThreatening "/Game/ChessGame/Materials/TileSelection_ValidMove.TileSelection_ValidMove" :Threaten 0 :Castling "/Game/ChessGame/Materials/TileSelection_Failed.TileSelection_Failed" :Failed "/Game/ChessGame/Materials/TileSelection_Failed.TileSelection_Failed"))
  (Development|SetHiddeninGame (Variables|Default|GetMarkerMesh) (or (Utilities|Enum|Equal(Enum) _selectionstate "None") (Utilities|Enum|Equal(Enum) _selectionstate "Threaten")) false))

(event MouseInput|EventActorOnClicked
  (params (ButtonPressed :type Key%20Structure))
  (Default|CallOnTileClicked self))

(fn ConstructionScript)